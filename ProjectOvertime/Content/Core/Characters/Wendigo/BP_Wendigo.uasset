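; BP_Wendigo is the Wendigo monster Blueprint for a scripted jumpscare that knocks out the first-person player.
; PlayScream roars, drives ABP_Wendigo from scream to run, switches off the player's flashlight and arms a Tick-polled follow.
; After a delay, FollowPlayer teleports it in front of the player, attacks, locks movement via MainGameMode, flickers the flashlight and calls KnockOut.
; The sight-based trigger for PlayScream is disconnected.
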(event Custom|PlayScream
  ;[1 1 1] Play Scream and Run Animation
  (bind _asabp_wendigo (Utilities|Casting|CastToABP_Wendigo (Components|SkeletalMesh|GetAnimInstance (Variables|Character|GetMesh))))
  (Variables|/Game/Core/Characters/Wendigo/ABP_Wendigo.ABP_Wendigo_C|SetOnScream _asabp_wendigo true)
  (Audio|PlaySound2D "/Game/Audios/SFX/SC_Monster_Roar.SC_Monster_Roar" 1.0 1.0 0.0 0 0)
  (Utilities|FlowControl|Delay 2.7)
  (Variables|/Game/Core/Characters/Wendigo/ABP_Wendigo.ABP_Wendigo_C|SetOnRun _asabp_wendigo true)
  (Variables|Default|SetCanFollowPlayer true)
  (Default|SwitchFlashLight (Variables|Default|GetAs%20BP%20First%20Person%20Movement) false))

(event Custom|FollowPlayer
  (bind _returnvalue (Game|GetPlayerCharacter 0))
  (bind _as_bp_first_person_movement (Variables|Default|GetAs%20BP%20First%20Person%20Movement))
  ;[1 1 1] Follow Player and Knockout event
  (Utilities|FlowControl|Delay 3.0)
  (Transformation|SetActorLocation (+ (Transformation|GetActorLocation _returnvalue) (* (Transformation|GetActorForwardVector _returnvalue) 1e+02)) false false)
  (Variables|Default|SetCanFollowPlayer false)
  (Audio|PlaySound2D "/Game/Audios/SFX/SC_Monster_Growl.SC_Monster_Growl" 1.0 1.0 0.0 0 0)
  (Audio|PlaySound2D "/Game/Audios/SFX/SC_Violin_Scare_Long.SC_Violin_Scare_Long" 1.0 1.0 0.0 0 0)
  (Variables|/Game/Core/Characters/Wendigo/ABP_Wendigo.ABP_Wendigo_C|SetOnAttack (stale Custom|PlayScream _asabp_wendigo) true)
  (bind _asmain_game_mode (Utilities|Casting|CastToMainGameMode (Game|GetGameMode)))
  (Variables|/Game/Core/Systems/MainGameMode.MainGameMode_C|SetcanMove _asmain_game_mode false)
  (Default|SwitchFlashLight _as_bp_first_person_movement true)
  (Default|FlashLightFlicking _as_bp_first_person_movement)
  (Utilities|FlowControl|Delay 1.3)
  (Audio|PlaySound2D "/Game/Audios/SFX/SC_Body_Hit.SC_Body_Hit" 1.0 1.0 0.0 0 0)
  (Development|PrintString "Hit")
  (Default|KnockOut (Variables|Default|GetAs%20BP%20First%20Person%20Movement)))

(event EventBeginPlay
  ;[1 1 1] Init
  (bind _asbp_first_person_movement (Utilities|Casting|CastToBP_FirstPersonMovement (Game|GetPlayerCharacter 0)))
  (Variables|Default|SetAs%20BP%20First%20Person%20Movement _asbp_first_person_movement))

(event EventTick
  (params (DeltaSeconds :type Float%20%28single-precision%29))
  ;[1 1 1] Check if it detects Player
  (if (Variables|Default|GetCanFollowPlayer)
    (CallFunction|FollowPlayer)))

(fn ConstructionScript)