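; Inventory component, by its AC_ prefix, that stores item data structs in a map keyed by item name.
; Adding an item inserts a new entry or increments the stored Amount by one if the name exists.
; Removal decrements based on the passed struct's Amount, deleting the entry when it is one or less.
; ID-based lookup and removal scan the map values linearly, and debug prints report each add or remove.
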(event Custom|Test
  (Development|PrintString "Test"))

(event EventBeginPlay)

(event EventTick
  (params (DeltaSeconds :type Float%20%28single-precision%29)))

(fn ContainsItemName
  (params (item :type S%20Item%20Data%20Structure))
  (return (Utilities|Map|Contains (Variables|Default|GetInventory) (.Name (Utilities|Struct|BreakS_ItemData item)))))

(fn AddItemtoInventory
  (params (item :type S%20Item%20Data%20Structure))
  (if (CallFunction|ContainsItemName item)
    (CallFunction|IncreaseItemAmount item)
    (Development|PrintString "Existed item incremented")
    (else
      (Utilities|Map|Add (Variables|Default|GetInventory) (.Name (Utilities|Struct|BreakS_ItemData item)) item)
      (Development|PrintString "New Item Added"))))

(fn IncreaseItemAmount
  (params (item :type S%20Item%20Data%20Structure))
  (bind _output_get (LocalVariables|SetName (.Name (Utilities|Struct|BreakS_ItemData item))))
  (if (.ReturnValue (Utilities|Map|Find (Variables|Default|GetInventory) _output_get))
    (bind _result (Math|Integer|IncrementInt (.Amount (Utilities|Struct|BreakS_ItemData (.Value (Utilities|Map|Find (Variables|Default|GetInventory) _output_get)))))
      (:%20%20
        (bind _structout (Utilities|Struct|SetmembersinS_ItemData (.Value (Utilities|Map|Find (Variables|Default|GetInventory) _output_get)) _result))
        (Utilities|Map|Add (Variables|Default|GetInventory) (LocalVariables|GetName) _structout)))))

(fn RemoveItem
  (params (Item :type S%20Item%20Data%20Structure))
  (bind (_name _amount) (Utilities|Struct|BreakS_ItemData Item))
  (if (Utilities|Map|Contains (Variables|Default|GetInventory) _name)
    (if (> _amount 1)
      (bind _result (Math|Integer|DecrementInt _amount)
        (:%20%20
          (bind _structout (Utilities|Struct|SetmembersinS_ItemData Item _result))
          (Utilities|Map|Add (Variables|Default|GetInventory) (.Name (Utilities|Struct|BreakS_ItemData _structout)) _structout)
          (Development|PrintString "Decrease Item")))
      (else
        (Utilities|Map|Remove (Variables|Default|GetInventory) (.Name (Utilities|Struct|BreakS_ItemData Item)))
        (Development|PrintString "Remove Item")))))

(fn ContainsItemID
  (params (Id :type Integer))
  (bind _values (Utilities|Map|Values (Variables|Default|GetInventory)))
  (for _array_element _values
    (if (== (.Id (Utilities|Struct|BreakS_ItemData _array_element)) Id)
      (LocalVariables|SetResult true)
      (return (LocalVariables|GetResult))))
  (return (LocalVariables|GetResult)))

(fn RemoveItembyID
  (params (ItemID :type Integer))
  (bind _values (Utilities|Map|Values (Variables|Default|GetInventory)))
  (for _array_element _values
    (if (== (.Id (Utilities|Struct|BreakS_ItemData _array_element)) ItemID)
      (CallFunction|RemoveItem _array_element))))