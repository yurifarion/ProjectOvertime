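; BP_Poster_1 is a readable note pickup that loads its title, content, category and thumbnail from the ItemDataValues_ENG data table by Id at BeginPlay.
; Hovering toggles custom depth on its mesh as a highlight.
; Interacting shows the text through BP_HUD, sets reading mode and registers the note with MainGameMode, then destroys the actor.
; GetItemData packs it as item data with a hardcoded category, ignoring the loaded one.
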(event Custom|GetDataFromMasterData
  ;[1 1 1] Get data from master data
  (bind _returnvalue (Utilities|GetDataTableRow "/Game/Core/MasterData/ItemDataValues_ENG.ItemDataValues_ENG" (Utilities|String|StringToName (Utilities|String|ToString(Integer) (Variables|Default|Getid))))
    (:then
      (Utilities|FlowControl|Sequence
        (:then_0
          (Variables|Default|SetTitle (Utilities|Text|ToText(String) (.Name (Utilities|Struct|BreakS_ItemData _returnvalue)))))
        (:then_1
          (Variables|Default|SetContent (.Description (Utilities|Struct|BreakS_ItemData _returnvalue))))
        (:then_2
          (Variables|Default|SetCategory (.Category (Utilities|Struct|BreakS_ItemData _returnvalue))))
        (:then_3
          (Variables|Default|SetThumbId (.ThumbId (Utilities|Struct|BreakS_ItemData _returnvalue))))))
    (:RowNotFound
      (Development|PrintString "item not found on master data"))))

(event EventBeginPlay
  (CallFunction|GetDatafromMasterData))

(event Collision|EventActorBeginOverlap
  (params (OtherActor :type Actor%20Object%20Reference)))

(event EventTick
  (params (DeltaSeconds :type Float%20%28single-precision%29)))

(event EventInteracted
  ;[1 1 1] Get Interacted
  (bind _asbp_hud (Utilities|Casting|CastToBP_HUD (HUD|GetHUD (Game|GetPlayerController 0))))
  (Default|ShowReadableFile _asbp_hud (Variables|Default|GetContent) (Variables|Default|GetTitle))
  (bind _asmain_game_mode (Utilities|Casting|CastToMainGameMode (Game|GetGameMode)))
  (Default|SetReadingMode _asmain_game_mode true)
  (Default|PickNoteItem _asmain_game_mode self)
  (CallFunction|OnPicked))

(event EventOnPicked
  ;[1 1 1] On Picked
  (Default|CallOnPickedEvent)
  (Actor|DestroyActor))

(event EventOnMouseExit
  ;[1 1 1] On Mouse Exit
  (Rendering|SetRenderCustomDepth (Variables|Default|GetStaticMeshModel) false))

(event EventOnMouseEnter
  ;[1 1 1] On Mouse Enter
  (Rendering|SetRenderCustomDepth (Variables|Default|GetStaticMeshModel) true))

(event EventOnHoverEnter
  (CallFunction|OnMouseEnter))

(event EventOnHoverExit
  (CallFunction|OnMouseExit))

(fn ConstructionScript)

(fn R
  (return (Utilities|Struct|MakeS_ItemData (Variables|Default|Getid) (Utilities|String|ToString(Text) (Variables|Default|GetTitle)) "NewEnumerator1" 1 (Variables|Default|GetContent))))

(fn GetItemData
  (return (Utilities|Struct|MakeS_ItemData (Variables|Default|Getid) (Utilities|String|ToString(Text) (Variables|Default|GetTitle)) "NewEnumerator1" 1 (Variables|Default|GetContent) (Variables|Default|GetThumbId))))