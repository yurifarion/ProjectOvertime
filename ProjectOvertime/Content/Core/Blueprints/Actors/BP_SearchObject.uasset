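; BP_SearchObject is a searchable item actor that the player hovers over and picks up.
; On BeginPlay it loads item fields by Id from the English item data table and creates a hidden outline-material mesh copy.
; Box cursor events toggle custom depth, the hand cursor and the game mode's current SearchObject.
; OnPicked passes the item data, amount one, to BP_HUD's detail display and destroys the actor.
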(event OnBeginCursorOver(Box)
  (params (TouchedComponent :type Primitive%20Component%20Object%20Reference))
  ;[1 1 1] Box Listener
  (CallFunction|OnMouseEnter))

(event OnEndCursorOver(Box)
  (params (TouchedComponent :type Primitive%20Component%20Object%20Reference))
  ;[1 1 1] Box Listener
  (CallFunction|OnMouseExit))

(event Custom|Set%20Outline%20Object
  (bind _objectsm (Variables|Default|GetObjectSM))
  ;[1 1 1] Set Outline FX
  (bind _returnvalue (AddComponent|AddStaticMeshComponent false (Transformation|GetRelativeTransform _objectsm)))
  (bind _output_get (Variables|Default|SetAdd%20Static%20Mesh _returnvalue))
  (Components|StaticMesh|SetStaticMesh _output_get (Variables|/Script/Engine.StaticMeshComponent|GetStaticMesh _objectsm))
  (Rendering|Material|SetMaterial (Variables|Default|GetAdd%20Static%20Mesh) 0 "/Game/Res/Material/M_Outline_Inst.M_Outline_Inst")
  (Rendering|Material|SetMaterial (Variables|Default|GetAdd%20Static%20Mesh) 1 "/Game/Res/Material/M_Outline_Inst.M_Outline_Inst")
  (Rendering|SetVisibility (Variables|Default|GetAdd%20Static%20Mesh) false false))

(event Custom|GetDataFromMasterData
  ;[1 1 1] Get data from master data
  (bind _returnvalue (Utilities|GetDataTableRow "/Game/Core/MasterData/ItemDataValues_ENG.ItemDataValues_ENG" (Utilities|String|StringToName (Utilities|String|ToString(Integer) (Variables|Default|GetId))))
    (:then
      (Utilities|FlowControl|Sequence
        (:then_0
          (Variables|Default|SetName (.Name (Utilities|Struct|BreakS_ItemData _returnvalue))))
        (:then_1
          (Variables|Default|SetCategory (.Category (Utilities|Struct|BreakS_ItemData _returnvalue))))
        (:then_2
          (Variables|Default|SetDescription (.Description (Utilities|Struct|BreakS_ItemData _returnvalue))))
        (:then_3
          (Variables|Default|SetThumbId (.ThumbId (Utilities|Struct|BreakS_ItemData _returnvalue))))))
    (:RowNotFound
      (Development|PrintString "item not found on master data"))))

(event EventOnPicked
  ;[1 1 1] On Picked
  (bind _asbp_hud (Utilities|Casting|CastToBP_HUD (HUD|GetHUD (Game|GetPlayerController 0))))
  (bind _itemdata (CallFunction|GetItemData))
  (Default|ShowItemDetail _asbp_hud _itemdata)
  (Actor|DestroyActor)
  (Variables|/Script/Engine.PlayerController|SetCurrentMouseCursor (Game|GetPlayerController 0) "Default"))

(event EventBeginPlay
  ;[1 1 1] Init
  (Utilities|IsValid self
    (:Is%20Valid
      (bind _asmain_game_mode (Utilities|Casting|CastToMainGameMode (Game|GetGameMode)))
      (Variables|Default|SetAs%20Main%20Game%20Mode _asmain_game_mode)
      (CallFunction|SetOutlineObject)
      (CallFunction|GetDatafromMasterData))))

(event EventOnMouseExit
  ;[1 1 1] Object Over Exit
  (Rendering|SetRenderCustomDepth (Variables|Default|GetObjectSM) false)
  (Variables|/Game/Core/Systems/MainGameMode.MainGameMode_C|SetSearchObject (Variables|Default|GetAs%20Main%20Game%20Mode) 0)
  (Variables|/Script/Engine.PlayerController|SetCurrentMouseCursor (Game|GetPlayerController 0) "Default"))

(event EventOnMouseEnter
  (bind _returnvalue (Game|GetPlayerController 0))
  ;[1 1 1] Object Over
  (Rendering|SetRenderCustomDepth (Variables|Default|GetObjectSM) true)
  (Variables|/Game/Core/Systems/MainGameMode.MainGameMode_C|SetSearchObject (Variables|Default|GetAs%20Main%20Game%20Mode) self)
  (Input|SetInputModeGameOnly _returnvalue false)
  (Variables|/Script/Engine.PlayerController|SetCurrentMouseCursor _returnvalue "Hand"))

(fn ConstructionScript)

(fn GetItemData
  (return (Utilities|Struct|MakeS_ItemData (Variables|Default|GetId) (Variables|Default|GetName) (Variables|Default|GetCategory) 1 (Variables|Default|GetDescription) (Variables|Default|GetThumbId))))