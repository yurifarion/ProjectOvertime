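; Interactable elevator that triggers the Wendigo endgame sequence, showing a "Use Elevator" prompt widget while hovered.
; Interaction checks the player's inventory for a required item and the IsEndGame flag, playing a failure sound if either is missing.
; On success it toggles tagged objects through MainGameMode, spawns the Wendigo and starts suspense music.
; After a delay, a one-shot event makes the Wendigo scream, then switches off the WendigoItem objects.
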(event Custom|EndLevelEvent
  (if (Variables|Default|GetIsEndGame)
    (bind _asmain_game_mode (Utilities|Casting|CastToMainGameMode (Game|GetGameMode)))
    (Development|PrintString "TODO: Scream")
    (Utilities|IsValid (Variables|/Game/Core/Systems/MainGameMode.MainGameMode_C|GetWendigoChar _asmain_game_mode)
      (:Is%20Valid
        (Utilities|FlowControl|DoOnce false
          (:Completed
            (bind _asbp_wendigo (Utilities|Casting|CastToBP_Wendigo (Variables|/Game/Core/Systems/MainGameMode.MainGameMode_C|GetWendigoChar _asmain_game_mode)))
            (Default|PlayScream _asbp_wendigo)
            (Utilities|FlowControl|Delay 1.0)
            (Default|SwitchObjects _asmain_game_mode false "WendigoItem")))))))

(event EventBeginPlay
  (bind _aswbp_interactable (Utilities|Casting|CastToWBP_Interactable (UserInterface|GetUserWidgetObject (Variables|Default|GetWidget))))
  (Default|ChangeText _aswbp_interactable "Use Elevator")
  (Rendering|SetVisibility (Variables|Default|GetWidget) false false))

(event Collision|EventActorBeginOverlap
  (params (OtherActor :type Actor%20Object%20Reference)))

(event EventTick
  (params (DeltaSeconds :type Float%20%28single-precision%29)))

(event EventOnHoverExit
  (Rendering|SetVisibility (Variables|Default|GetWidget) false false))

(event EventOnHoverEnter
  (Rendering|SetVisibility (Variables|Default|GetWidget) true false))

(event EventInteracted
  (bind _asbp_first_person_movement (Utilities|Casting|CastToBP_FirstPersonMovement (Game|GetPlayerCharacter 0)))
  (bind _bool (Default|ContainsItemID (Variables|/Game/Core/Characters/BP_FirstPersonMovement.BP_FirstPersonMovement_C|GetAC_Inventory _asbp_first_person_movement) 7))
  (if _bool
    (if (Variables|Default|GetIsEndGame)
      (Development|PrintString "Spawn Wendigo")
      (Audio|PlaySoundatLocation "/Game/Audios/SFX/SC_Elevator_Button.SC_Elevator_Button" (Transformation|GetActorLocation) "0, 0, 0" 1.0 1.0 0.0 "/Game/Audios/SFX/Attenuation/SA_Default.SA_Default" 0 0 0)
      (bind _asmain_game_mode (Utilities|Casting|CastToMainGameMode (Game|GetGameMode)))
      (Default|SwitchObjects _asmain_game_mode false "HiddenLight")
      (Default|SwitchObjects _asmain_game_mode true "OffDevice")
      (Default|SwitchObjects _asmain_game_mode true "WendigoItem")
      (Default|SpawnWendigo _asmain_game_mode "-18944.147826,-15470.453042,87.995516" "0.000000,90.000000,0.000000")
      (Audio|SpawnSound2D "/Game/Audios/AMB/BMG_Suspense_01.BMG_Suspense_01" 1.0 1.0 0.0 0)
      (Utilities|FlowControl|Delay 3.0)
      (CallFunction|EndLevelEvent)
      (else
        (Audio|PlaySound2D "/Game/Audios/VO/SC_Elevator_Without_Power.SC_Elevator_Without_Power" 1.0 1.0 0.0 0 0)))
    (else
      (Audio|PlaySound2D "/Game/Audios/VO/SC_Elevator_Without_Bag.SC_Elevator_Without_Bag" 1.0 1.0 0.0 0 0))))

(fn ConstructionScript)