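; BP_FlickyLight is a rect light actor that can be switched into and out of a flickering state.
; TurnonFlickering assigns a dynamic instance of FlickerLight_Inst as the light function material with FlickerEnable on, then calls TurnoffFlickering after the given duration.
; A zero or negative duration leaves the flicker running.
; Each toggle creates a fresh material instance rather than reusing one.
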(event Custom|Turn%20on%20Flickering
  (params (Duration :type Float%20%28double-precision%29))
  (bind _returnvalue (Rendering|Material|CreateDynamicMaterialInstance "/Game/Res/Material/FlickerLight_Inst.FlickerLight_Inst" "None" "None" :!class /Script/Engine.KismetMaterialLibrary))
  (Rendering|Material|SetScalarParameterValue _returnvalue "FlickerEnable" 1.0 :!class /Script/Engine.MaterialInstanceDynamic)
  (Rendering|Components|Light|SetLightFunctionMaterial (Variables|Default|GetRectLight) _returnvalue)
  (if (not (<= Duration 0.0))
    (Utilities|FlowControl|Delay Duration)
    (CallFunction|TurnOffFlickering)))

(event Custom|Turn%20off%20Flickering
  (bind _returnvalue (Rendering|Material|CreateDynamicMaterialInstance "/Game/Res/Material/FlickerLight_Inst.FlickerLight_Inst" "None" "None" :!class /Script/Engine.KismetMaterialLibrary))
  (Rendering|Material|SetScalarParameterValue _returnvalue "FlickerEnable" 0.0 :!class /Script/Engine.MaterialInstanceDynamic)
  (Rendering|Components|Light|SetLightFunctionMaterial (Variables|Default|GetRectLight) _returnvalue))

(fn ConstructionScript)