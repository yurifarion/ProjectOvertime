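; Interactable door actor that opens and closes by rotating its mesh with MoveComponentTo, with sounds and an optional lock.
; Interacting while locked requires the matching KeyID in the player's inventory or the game mode's key-master flag.
; Unlocking can also skip the key check, and always calls item removal for KeyID.
; A hover-only widget shows Unlock, Open or Close and registers with the HUD's gameplay widget list.
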(event Custom|Open%20Door
  ;[1 1 1] Open Door
  (if (Variables|Default|GetisLocked)
    (CallFunction|IsLockedEvent)
    (else
      (Audio|PlaySoundatLocation "/Game/Audios/SFX/SC_Open_Door.SC_Open_Door" (Transformation|GetActorLocation) "0, 0, 0" 1.0 1.0 0.0 0 0 0 0)
      (Components|MoveComponentTo (Variables|Default|GetDoor_SM) "0, 0, 0" (Variables|Default|GetAngleToOpen) false false 0.8 false)
      (Variables|Default|SetisOpen true)
      (CallFunction|UpdatePromptText))))

(event Custom|IsLockedEvent
  ;[1 1 1] Is Locked
  (Development|PrintString "The door is locked"))

(event Custom|Unlock%20Door
  (params (No%20Key :type Boolean))
  (bind _keyid (Variables|Default|GetKeyID))
  ;[1 1 1] Unlock Door
  (bind _asbp_first_person_movement (Utilities|Casting|CastToBP_FirstPersonMovement (Game|GetPlayerCharacter 0)))
  (if No%20Key
    (Variables|Default|SetisLocked false :!label _label)
    (Development|PrintString "Door Unlocked")
    (CallFunction|UpdatePromptText)
    (Default|RemoveItembyID (Variables|/Game/Core/Characters/BP_FirstPersonMovement.BP_FirstPersonMovement_C|GetAC_Inventory _asbp_first_person_movement) _keyid)
    (Audio|PlaySoundatLocation "/Game/Audios/SFX/SC_Unlock_Door.SC_Unlock_Door" (Transformation|GetActorLocation) "0, 0, 0" 1.0 1.0 0.0 0 0 0 0)
    (else
      (bind _bool (Default|ContainsItemID (Variables|/Game/Core/Characters/BP_FirstPersonMovement.BP_FirstPersonMovement_C|GetAC_Inventory _asbp_first_person_movement) _keyid))
      (if _bool
        (goto _label)
        (else
          (bind _asmain_game_mode (Utilities|Casting|CastToMainGameMode (Game|GetGameMode)))
          (if (Variables|/Game/Core/Systems/MainGameMode.MainGameMode_C|GetIsKeyMaster _asmain_game_mode)
            (goto _label)
            (else
              (CallFunction|IsLockedEvent))))))))

(event Custom|UpdatePromptText
  ;[1 1 1] Update Prompt text
  (bind _aswbp_interactable (Utilities|Casting|CastToWBP_Interactable (UserInterface|GetUserWidgetObject (Variables|Default|GetWidget))))
  (if (Variables|Default|GetisLocked)
    (Default|ChangeText _aswbp_interactable "Unlock")
    (elif (Variables|Default|GetisOpen)
      (Default|ChangeText _aswbp_interactable "Close")
      (else
        (Default|ChangeText _aswbp_interactable "Open")))))

(event Custom|Close%20Door
  ;[1 1 1] Close Door
  (if (not (Variables|Default|GetisLocked))
    (Components|MoveComponentTo (Variables|Default|GetDoor_SM) "0, 0, 0" "0, 0, 0" false false 0.8 false)
    (Variables|Default|SetisOpen false)
    (CallFunction|UpdatePromptText)
    (Audio|PlaySoundatLocation "/Game/Audios/SFX/SC_Close_Door.SC_Close_Door" (Transformation|GetActorLocation) "0, 0, 0" 1.0 1.0 0.0 0 0 0 0)))

(event EventBeginPlay
  (bind _widget (Variables|Default|GetWidget))
  (CallFunction|UpdatePromptText)
  (Rendering|SetVisibility _widget false false)
  (bind _asbp_hud (Utilities|Casting|CastToBP_HUD (HUD|GetHUD (Game|GetPlayerController 0))))
  (bind _asbpi_in_game_wbp (Utilities|Casting|CastToBPI_InGameWBP (UserInterface|GetUserWidgetObject _widget)))
  (Utilities|Array|Add (Variables|/Game/Core/Blueprints/HUD/BP_HUD.BP_HUD_C|GetGameplayWB _asbp_hud) _asbpi_in_game_wbp))

(event Collision|EventActorBeginOverlap
  (params (OtherActor :type Actor%20Object%20Reference)))

(event EventTick
  (params (DeltaSeconds :type Float%20%28single-precision%29)))

(event EventOnHoverEnter
  (Rendering|SetVisibility (Variables|Default|GetWidget) true false))

(event EventOnHoverExit
  (Rendering|SetVisibility (Variables|Default|GetWidget) false false))

(event EventInteracted
  ;[1 1 1] Interacted
  (if (Variables|Default|GetisLocked)
    (CallFunction|UnlockDoor false)
    (elif (Variables|Default|GetisOpen)
      (CallFunction|CloseDoor)
      (else
        (CallFunction|OpenDoor)))))

(fn ConstructionScript)