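; BP_SearchTable is an interactable table that switches the game into search mode with a dedicated camera view.
; When interacted with outside search mode, it plays a camera-move sound, blends the view to its BP_CameraLocation child actor, enables search mode on MainGameMode and clears its highlight.
; Hover events toggle custom depth on the table mesh for highlighting, which only turns on outside search mode.
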(event EventBeginPlay)

(event Collision|EventActorBeginOverlap
  (params (OtherActor :type Actor%20Object%20Reference)))

(event EventTick
  (params (DeltaSeconds :type Float%20%28single-precision%29)))

(event EventInteracted
  ;[1 1 1] Interacted
  (bind _asmain_game_mode (Utilities|Casting|CastToMainGameMode (Game|GetGameMode)))
  (if (not (Variables|/Game/Core/Systems/MainGameMode.MainGameMode_C|GetOnSearchMode _asmain_game_mode))
    (bind _asbp_camera_location (Utilities|Casting|CastToBP_CameraLocation (Variables|/Script/Engine.ChildActorComponent|GetChildActor (Variables|Default|GetCameraPos))))
    (Audio|PlaySound2D "/Game/Audios/SFX/SC_Camera_Move.SC_Camera_Move" 1.0 1.0 0.0 0 0)
    (Game|Player|SetViewTargetwithBlend (Game|GetPlayerController 0) _asbp_camera_location 1.0 "VTBlend_Cubic" 0.0 false)
    (Default|SetSearchMode _asmain_game_mode true)
    (CallFunction|OnHoverExit)))

(event EventOnHoverEnter
  ;[1 1 1] On Hover Enter
  (bind _asmain_game_mode (Utilities|Casting|CastToMainGameMode (Game|GetGameMode)))
  (if (not (Variables|/Game/Core/Systems/MainGameMode.MainGameMode_C|GetOnSearchMode _asmain_game_mode))
    (Rendering|SetRenderCustomDepth (Variables|Default|GetSM_Object) true)))

(event EventOnHoverExit
  ;[1 1 1] On Hover Exit
  (Rendering|SetRenderCustomDepth (Variables|Default|GetSM_Object) false))

(fn ConstructionScript)