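; BP_SearchOpenable is an interactable door that opens for a close-up search mode.
; Hovering toggles an "Open" prompt widget, which BeginPlay also registers with the HUD's gameplay widgets.
; Interacting outside search mode blends the view to a child camera actor, enables search mode and registers the door as SearchDoor on MainGameMode.
; OpenDoor and CloseDoor rotate the door with MoveComponentTo only when unlocked, though the camera switch ignores the lock.
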(event Custom|Open%20Door
  (bind _opendoor (Variables|Default|GetOpenDoor))
  ;[1 1 1] Open Door
  (CallFunction|OnHoverExit)
  (if (not (Variables|Default|GetIs%20Locked))
    (Components|MoveComponentTo _opendoor (Variables|/Script/Engine.SceneComponent|GetRelativeLocation _opendoor) "0.000000,-90.000000,0.000000" false false 1.0 false)
    (Variables|Default|SetIs%20Open true)))

(event Custom|Close%20Door
  (bind _opendoor (Variables|Default|GetOpenDoor))
  ;[1 1 1] Close Door
  (if (not (Variables|Default|GetIs%20Locked))
    (Components|MoveComponentTo _opendoor (Variables|/Script/Engine.SceneComponent|GetRelativeLocation _opendoor) "0, 0, 0" false false 1.0 false)
    (Variables|Default|SetIs%20Open false)))

(event EventBeginPlay
  (bind _widget (Variables|Default|GetWidget))
  (bind _returnvalue (UserInterface|GetUserWidgetObject _widget))
  (Rendering|SetVisibility _widget false false)
  (bind _asbp_hud (Utilities|Casting|CastToBP_HUD (HUD|GetHUD (Game|GetPlayerController 0))))
  (bind _asbpi_in_game_wbp (Utilities|Casting|CastToBPI_InGameWBP _returnvalue))
  (Utilities|Array|Add (Variables|/Game/Core/Blueprints/HUD/BP_HUD.BP_HUD_C|GetGameplayWB _asbp_hud) _asbpi_in_game_wbp)
  (bind _aswbp_interactable (Utilities|Casting|CastToWBP_Interactable _returnvalue))
  (Default|ChangeText _aswbp_interactable "Open"))

(event EventOnHoverExit
  (Rendering|SetVisibility (Variables|Default|GetWidget) false false))

(event EventOnHoverEnter
  (Rendering|SetVisibility (Variables|Default|GetWidget) true false))

(event EventInteracted
  ;[1 1 1] Interacted
  (bind _asmain_game_mode (Utilities|Casting|CastToMainGameMode (Game|GetGameMode)))
  (if (not (Variables|/Game/Core/Systems/MainGameMode.MainGameMode_C|GetOnSearchMode _asmain_game_mode))
    (bind _asbp_camera_location (Utilities|Casting|CastToBP_CameraLocation (Variables|/Script/Engine.ChildActorComponent|GetChildActor (Variables|Default|GetCamera%20Pos))))
    (Game|Player|SetViewTargetwithBlend (Game|GetPlayerController 0) _asbp_camera_location 1.0 "VTBlend_Linear" 0.0 false)
    (bind _asmain_game_mode_2 (Utilities|Casting|CastToMainGameMode (Game|GetGameMode)))
    (Default|SetSearchMode _asmain_game_mode_2 true)
    (CallFunction|OpenDoor)
    (Variables|/Game/Core/Systems/MainGameMode.MainGameMode_C|SetSearchDoor _asmain_game_mode_2 self)))

(fn ConstructionScript)