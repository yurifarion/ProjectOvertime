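; Interactable generator that the player restarts to turn the lights on, with looping, blackout and startup sounds.
; A hover prompt shows while the light is off; interacting first checks the player's inventory for the code item, then updates the prompt.
; The next interaction sets the light on, calls LightsOn and plays the start sound, resuming the loop after that sound's duration.
; EnterBlackout stops the loop and plays a blackout sound.
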(event Custom|EnterBlackout
  (Audio|Components|Audio|Stop (Variables|Default|GetGeneratorLoopSound))
  (Audio|PlaySoundatLocation "/Game/Audios/SFX/SC_Generator_Blackout.SC_Generator_Blackout" (Transformation|GetActorLocation) "0, 0, 0" 1.0 1.0 0.0 "/Game/Audios/SFX/Attenuation/SA_Generator.SA_Generator" 0 0 0))

(event Custom|Start%20Generator
  (bind _returnvalue (Audio|SpawnSoundatLocation "/Game/Audios/SFX/SC_Generator_Start.SC_Generator_Start" (Transformation|GetActorLocation) "0, 0, 0" 1.0 1.0 0.0 "/Game/Audios/SFX/Attenuation/SA_Generator.SA_Generator" 0))
  (Utilities|FlowControl|Delay (Variables|/Script/Engine.SoundBase|GetDuration (Variables|/Script/Engine.AudioComponent|GetSound _returnvalue)))
  (Audio|Components|Audio|Play (Variables|Default|GetGeneratorLoopSound) 0.0))

(event EventBeginPlay
  (bind _aswbp_interactable (Utilities|Casting|CastToWBP_Interactable (UserInterface|GetUserWidgetObject (Variables|Default|GetWidget))))
  (Default|ChangeText _aswbp_interactable "Insert Code")
  (Rendering|SetVisibility (Variables|Default|GetWidget) false false)
  (bind _returnvalue (Audio|SpawnSoundatLocation "/Game/Audios/SFX/SC_Generator_Loop.SC_Generator_Loop" (Transformation|GetActorLocation) "0, 0, 0" 1.0 1.0 0.0 "/Game/Audios/SFX/Attenuation/SA_Generator.SA_Generator" 0 false))
  (Variables|Default|SetGeneratorLoopSound _returnvalue))

(event Collision|EventActorBeginOverlap
  (params (OtherActor :type Actor%20Object%20Reference)))

(event EventTick
  (params (DeltaSeconds :type Float%20%28single-precision%29)))

(event EventInteracted
  (if (not (Variables|Default|GetLightOn))
    (if (Variables|Default|GetCodeInserted)
      (Development|PrintString "Turn Light On")
      (Variables|Default|SetLightOn true)
      (Default|CallLightson)
      (CallFunction|StartGenerator)
      (else
        (bind _asbp_first_person_movement (Utilities|Casting|CastToBP_FirstPersonMovement (Game|GetPlayerCharacter 0)))
        (bind _bool (Default|ContainsItemID (Variables|/Game/Core/Characters/BP_FirstPersonMovement.BP_FirstPersonMovement_C|GetAC_Inventory _asbp_first_person_movement) 8))
        (if _bool
          (Variables|Default|SetCodeInserted true)
          (bind _aswbp_interactable (Utilities|Casting|CastToWBP_Interactable (UserInterface|GetUserWidgetObject (Variables|Default|GetWidget))))
          (Default|ChangeText _aswbp_interactable "Turn on generator"))))))

(event EventOnHoverEnter
  (if (not (Variables|Default|GetLightOn))
    (Rendering|SetVisibility (Variables|Default|GetWidget) true false)))

(event EventOnHoverExit
  (Rendering|SetVisibility (Variables|Default|GetWidget) false false))

(fn ConstructionScript)