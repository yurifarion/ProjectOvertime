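; Main menu GameMode that sets up the menu scene, its UI intro and its audio on BeginPlay.
; It sets Game and UI input with the cursor hidden, plays night forest ambience and streams in the menu sublevel without blocking.
; A fixed delay, rather than a load callback, precedes the HUD widget's GameStart and LevelFadeIn calls.
; The main music starts after a further delay.
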(event EventBeginPlay
  (bind _returnvalue (Game|GetPlayerController 0))
  (Input|SetInputModeGameandUI _returnvalue 0 "DoNotLock" true false)
  (Variables|/Script/Engine.PlayerController|SetbShowMouseCursor _returnvalue false)
  (Audio|PlaySound2D "/Game/Audios/AMB/AMB_Forest_Night_Wind.AMB_Forest_Night_Wind" 1.0 1.0 0.0 0 0)
  (Game|LoadStreamLevel(byName) "MainMenuSubLevel" true)
  (Utilities|FlowControl|Delay 2.0)
  (bind _asbp_main_menu_hud (Utilities|Casting|CastToBP_MainMenuHUD (HUD|GetHUD (Game|GetPlayerController 0))))
  (Default|GameStart (Variables|/Game/Core/Blueprints/HUD/BP_MainMenuHUD.BP_MainMenuHUD_C|GetMainMenuWBP _asbp_main_menu_hud))
  (Default|LevelFadein (Variables|/Game/Core/Blueprints/HUD/BP_MainMenuHUD.BP_MainMenuHUD_C|GetMainMenuWBP _asbp_main_menu_hud))
  (Utilities|FlowControl|Delay 5.0)
  (Audio|PlaySound2D "/Game/Audios/AMB/BMG_Main_Music.BMG_Main_Music" 1.0 1.0 0.0 0 0))

(fn ConstructionScript)